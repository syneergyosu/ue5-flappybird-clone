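; Player controller for a Flappy Birds game that owns the main UI and relays game state to it.
; On BeginPlay it switches to game-only input and creates the main widget.
; Its events forward score and result values to the score and game-over sub-widgets.
; Showing or hiding the game-over panel also toggles the mouse cursor and UI-only versus game-only input.
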(event Custom|ShowUI
  ;[1 1 1] Show Main UI
  (bind _returnvalue (UserInterface|CreateWidget "/Game/_Main/Widgets/WB_Main.WB_Main_C"))
  (bind _output_get (Variables|Default|SetWB_MainRef _returnvalue))
  (UserInterface|Viewport|AddtoViewport _output_get 0))

(event Custom|UpdateScore
  (params (Score :type Integer))
  ;[1 1 1] Update Score UI
  (Default|UpdateScoreUI (Variables|/Game/_Main/Widgets/WB_Main.WB_Main_C|GetWB_Score (Variables|Default|GetWB_MainRef)) Score))

(event Custom|ShowGameOverUI
  (params (isVisible? :type Boolean))
  (bind _self self)
  (bind _wb_mainref (Variables|Default|GetWB_MainRef))
  (bind _wb_gameover (Variables|/Game/_Main/Widgets/WB_Main.WB_Main_C|GetWB_GameOver _wb_mainref))
  ;[1 1 1] Game Over UI
  (if isVisible?
    (Widget|SetVisibility _wb_gameover "Visible")
    (Variables|Default|SetbShowMouseCursor true)
    (Input|SetInputModeUIOnly _self 0 "DoNotLock" false)
    (else
      (Widget|SetVisibility _wb_gameover "Hidden")
      (Variables|Default|SetbShowMouseCursor false)
      (Input|SetInputModeGameOnly _self false))))

(event Custom|UpdateResultUI
  (params (CurrentScore :type Integer) (BestScore :type Integer))
  ;[1 1 1] Update Result UI
  (Default|UpdateResult (Variables|/Game/_Main/Widgets/WB_Main.WB_Main_C|GetWB_GameOver (Variables|Default|GetWB_MainRef)) CurrentScore BestScore))

(event EventBeginPlay
  ;[1 1 1] Focuses instantly onto the game and show main ui
  (Input|SetInputModeGameOnly self false)
  (CallFunction|ShowUI))

(fn ConstructionScript)

(fn GetControllerReference
  (return self))