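; BP_ScoreButton is a clickable 3D menu button that prints the player's best score from NewGameInstance.
; A click runs timeline-driven press and release motions through MoveButton, then after a short delay sets IsPressed and prints the score.
; MoveButton lerps from the mesh's current world location each update, with IsPressed choosing the offset size.
; Cursor hover swaps the button and base materials.
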(event OnClicked(SM_StartButton)
  (params (TouchedComponent :type Primitive%20Component%20Object%20Reference) (ButtonPressed :type Key%20Structure :default "None"))
  ;[1 1 1] On Clicked Play Button Animation And Show Player Score
  (CallFunction|ButtonDown)
  (Utilities|FlowControl|Delay 0.4)
  (Variables|Default|SetisPressed? true)
  (bind _asnew_game_instance (Utilities|Casting|CastToNewGameInstance (Game|GetGameInstance)))
  (Development|PrintString (Utilities|String|ToString(Integer) (Variables|/Game/Blueprints/NewGameInstance.NewGameInstance_C|GetBestScore _asnew_game_instance))))

(event OnBeginCursorOver(SM_StartButton)
  (params (TouchedComponent :type Primitive%20Component%20Object%20Reference))
  ;[1 1 1] Set Material On Hover
  (Rendering|Material|SetMaterial (Variables|Default|GetSM_StartButton) 0 "/Game/_Main/Assets/UI/Buttons/Score/Material/M_HoverScore.M_HoverScore"))

(event OnEndCursorOver(SM_StartButton)
  (params (TouchedComponent :type Primitive%20Component%20Object%20Reference))
  ;[1 1 1] Set Material On Hover
  (Rendering|Material|SetMaterial (Variables|Default|GetSM_StartButton) 0 "/Game/_Main/Assets/UI/Buttons/Score/Material/M_BaseScore.M_BaseScore"))

(event Custom|ButtonDown
  ;[1 1 1] Button Animation
  (bind _alpha (Timeline|T_Move Play)
    (:Update
      (CallFunction|MoveButton _alpha (Variables|Default|GetSM_StartButton) (Math|Vector|SelectVector "4.500000,0.000000,0.000000" "1.000000,0.000000,0.000000" (Variables|Default|GetisPressed?)))
      (Utilities|FlowControl|Delay 0.2)
      (CallFunction|ButtonUp))))

(event Custom|ButtonUp
  ;[1 1 1] Button Animation
  (bind _alpha (Timeline|Timeline Play)
    (:Update
      (CallFunction|MoveButton _alpha (Variables|Default|GetSM_StartButton) (Math|Vector|SelectVector "-4.500000,0.000000,0.000000" "-1.000000,0.000000,0.000000" (Variables|Default|GetisPressed?))))))

(fn ConstructionScript)

(fn MoveButton
  (params (Alpha :type Float%20%28single-precision%29) (Target :type Scene%20Component%20Object%20Reference) (Location :type Vector))
  (bind _returnvalue (Transformation|GetWorldLocation Target))
  (Transformation|SetWorldLocation Target (Math|Vector|Lerp(Vector) _returnvalue (+ _returnvalue Location) Alpha) false false))