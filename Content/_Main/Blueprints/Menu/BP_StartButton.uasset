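; BP_StartButton is a clickable 3D menu button that animates a press and then opens the L_World level.
; Clicking the mesh runs ButtonDown, then ButtonUp and the level load after short delays.
; Two timelines drive MoveButton, which shifts the mesh along world X in opposite directions.
; MoveButton lerps from the mesh's current location on every update, so the offset accumulates rather than tracking a fixed start point.
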(event OnClicked(SM_StartButton)
  (params (TouchedComponent :type Primitive%20Component%20Object%20Reference) (ButtonPressed :type Key%20Structure :default "None"))
  (CallFunction|ButtonDown)
  (Utilities|FlowControl|Delay 0.2)
  (CallFunction|ButtonUp)
  (Utilities|FlowControl|Delay 0.4)
  (Game|OpenLevel(byName) "L_World"))

(event Custom|ButtonDown
  (bind _alpha (Timeline|T_Move Play)
    (:Update
      (CallFunction|MoveButton _alpha (Variables|Default|GetSM_StartButton) "1.000000,0.000000,0.000000"))))

(event Custom|ButtonUp
  (bind _alpha (Timeline|Timeline Play)
    (:Update
      (CallFunction|MoveButton _alpha (Variables|Default|GetSM_StartButton) "-1.000000,0.000000,0.000000"))))

(fn ConstructionScript)

(fn MoveButton
  (params (Alpha :type Float%20%28single-precision%29) (Target :type Scene%20Component%20Object%20Reference) (Location :type Vector))
  (bind _returnvalue (Transformation|GetWorldLocation Target))
  (Transformation|SetWorldLocation Target (Math|Vector|Lerp(Vector) _returnvalue (+ _returnvalue Location) Alpha) false false))