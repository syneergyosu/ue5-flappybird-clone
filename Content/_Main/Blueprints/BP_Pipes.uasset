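; BP_Pipes is a moving pipe obstacle that awards a point when the player overlaps its box, like a Flappy Bird pipe.
; On BeginPlay a timeline drives the mesh's world Y with sweep, and a delay started from its update destroys the actor seconds later.
; Only the pipe rolled 180 degrees (top) scores, fetching player and controller through reference messages to increment and update the score.
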(event OnComponentBeginOverlap(Box)
  (params (OverlappedComponent :type Primitive%20Component%20Object%20Reference) (OtherActor :type Actor%20Object%20Reference) (OtherComp :type Primitive%20Component%20Object%20Reference) (OtherBodyIndex :type Integer) (bFromSweep :type Boolean) (SweepResult :type Hit%20Result%20Structure%20%28by%20ref%29))
  ;[1 1 1] If a player overlaps the box collision add one score
  (if (== (.roll (Transformation|GetWorldRotation (Variables|Default|GetStaticMesh))) 1.8e+02) ; Top Pipe?
    (bind _reference (Class|BPIPlayerReference|GetPlayerReference(Message) OtherActor))
    (Utilities|IsValid _reference
      (:Is%20Valid
        (bind _output_get (Variables|/Game/_Main/Blueprints/BP_ThirdPersonCharacter.BP_ThirdPersonCharacter_C|SetScore _reference (+ (Variables|/Game/_Main/Blueprints/BP_ThirdPersonCharacter.BP_ThirdPersonCharacter_C|GetScore _reference) 1)))
        (bind _reference_2 (Class|BPIControllerReference|GetControllerReference(Message) (Game|GetPlayerController 0)))
        (Default|UpdateScore _reference_2 _output_get)))))

(event Custom|PipeMoving
  (bind _staticmesh (Variables|Default|GetStaticMesh))
  (bind _returnvalue (Transformation|GetWorldLocation _staticmesh))
  (bind (_x _y _z) (Math|Vector|BreakVector _returnvalue))
  ;[1 1 1] Pipes moving to the left
  (bind _alpha (Timeline|T_Move PlayFromStart)
    (:Update
      (Transformation|SetWorldLocation _staticmesh (Math|Vector|MakeVector _x _alpha _z) true false)
      (Utilities|FlowControl|Delay 7.0)
      (Actor|DestroyActor))))

(event EventBeginPlay
  (CallFunction|PipeMoving))

(fn ConstructionScript)