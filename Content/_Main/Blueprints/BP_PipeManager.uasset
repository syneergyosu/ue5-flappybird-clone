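; BP_PipeManager spawns pairs of BP_Pipes obstacles at a fixed Y position, starting on BeginPlay.
; BottomPipe loops on a two-second Delay, spawning a pipe at random height and passing its mesh's world Z to TopPipe.
; TopPipe spawns a flipped pipe at a fixed offset above that height, intended to keep the gap constant.
; TopPipe also re-calls itself after its own Delay, alongside the BottomPipe loop.
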(event Custom|BottomPipe
  ;[1 1 1] Spawn Pipes and make sure there is a same gap between them
  (bind _returnvalue (Game|SpawnActorfromClass "/Game/_Main/Blueprints/BP_Pipes.BP_Pipes_C" (Math|Transform|MakeTransform (Math|Vector|MakeVector 0.0 1.55e+03 (Math|Random|RandomFloatinRange 0.0 4e+02)) "0, 0, 0" "1.000000,1.000000,1.000000") "AdjustIfPossibleButAlwaysSpawn" "MultiplyWithRoot" 0 0 :!label _label))
  (bind _output_get (Variables|Default|SetBottomStaticMesh (Variables|/Game/_Main/Blueprints/BP_Pipes.BP_Pipes_C|GetStaticMesh _returnvalue)))
  (CallFunction|TopPipe (.z (Transformation|GetWorldLocation _output_get)))
  (Utilities|FlowControl|Delay 2.0)
  (goto _label))

(event Custom|TopPipe
  (params (Height :type Float%20%28double-precision%29))
  (bind _returnvalue (+ Height 1.3e+03))
  (bind _returnvalue_2 (Math|Vector|MakeVector 0.0 1.55e+03 _returnvalue))
  ;[1 1 1] Spawn Pipes and make sure there is a same gap between them
  (Variables|Default|SetTopPipeLoc _returnvalue_2)
  (Game|SpawnActorfromClass "/Game/_Main/Blueprints/BP_Pipes.BP_Pipes_C" (Math|Transform|MakeTransform _returnvalue_2 "0.000000,0.000000,180.000000" "1.000000,1.000000,1.000000") "AdjustIfPossibleButAlwaysSpawn" "MultiplyWithRoot" 0 0)
  (Utilities|FlowControl|Delay 2.0)
  (CallFunction|TopPipe (+ (Variables|Default|GetZ) 1.3e+03)))

(event EventBeginPlay
  ;[1 1 1] Spawn Both Pipes
  (CallFunction|BottomPipe)
  (CallFunction|TopPipe (+ (Variables|Default|GetZ) 1.3e+03)))

(fn ConstructionScript)